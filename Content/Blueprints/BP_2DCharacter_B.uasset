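; BP_2DCharacter_B is a 2D playable character, shown as a golem ball while disabled, with its own speed and health values set in the construction script.
; It starts with movement disabled; Enable and Disable functions toggle walking and the IsEnabled flag.
; While enabled, Tick sets the idle flipbook every frame.
; Pressing C makes player controller 0 possess BP_2DCharacter_A, without calling either toggle function here.
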(event EventBeginPlay
  (|CallParentFunction)
  (Utilities|FlowControl|Sequence
    (:then_0
      (CallFunction|DisablePlayer))
    (:then_1
      (Sprite|SetFlipbook (Variables|Default|GetSprite) "/Game/Assets/Flipbooks/FB_GolemBall.FB_GolemBall"))))

(event Collision|EventActorBeginOverlap
  (params (OtherActor :type Actor%20Object%20Reference))
  (|CallParentFunction OtherActor) ; This node is disabled and will not be called.\nDrag off pins to build functionality.
)

(event EventTick
  (params (DeltaSeconds :type Float%20%28single-precision%29))
  (|CallParentFunction DeltaSeconds)
  (if (Variables|Default|GetIsEnabled)
    (Sprite|SetFlipbook (Variables|Default|GetSprite) "/Game/Assets/Flipbooks/FB_PlayerB_Idle.FB_PlayerB_Idle")))

(event Input|KeyboardEvents|C
  (params (Key :type Key%20Structure))
  (:Pressed
    ;[1 1 1] Change Character
    (bind _returnvalue (Actor|GetActorOfClass "/Game/Blueprints/BP_2DCharacter_A.BP_2DCharacter_A_C"))
    (Pawn|Possess (Game|GetPlayerController 0) _returnvalue)))

(fn ConstructionScript
  (|CallParentFunction)
  (Variables|Default|SetWalkSpeed 1e+02)
  (Variables|Default|SetSprintSpeed 5e+02)
  (Variables|Default|SetMaxHealth 1e+03))

(fn DisablePlayer
  (Pawn|Components|CharacterMovement|DisableMovement (Variables|Character|GetCharacterMovement))
  (Variables|Default|SetIsEnabled false))

(fn EnablePlayer
  (Pawn|Components|CharacterMovement|SetMovementMode (Variables|Character|GetCharacterMovement) "MOVE_Walking" 0)
  (Variables|Default|SetIsEnabled true))