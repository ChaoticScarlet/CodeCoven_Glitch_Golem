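; BP_PlayerB is a side-view Paper2D golem character that swaps possession to BP_PlayerA on C.
; It starts as an immobile ball, and T flip-flops between disabling and enabling it, though the first press repeats the disabled state.
; Input drives X-axis movement, jumping and sprinting.
; Tick grid-snaps the spring arm for a pixel-aligned camera, turns the controller toward horizontal velocity and reapplies the idle flipbook while enabled.
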(event Custom|UpdateDirection
  (Utilities|IsValid (Pawn|GetController)
    (:Is%20Valid
      (Math|Float|CompareFloat (.X (Math|Vector|BreakVector (Variables|/Script/Engine.MovementComponent|GetVelocity (Variables|Character|GetCharacterMovement)))) 0.0
        (:>
          (Pawn|SetControlRotation (Pawn|GetController) (Math|Rotator|MakeRotator 0.0 0.0 0.0)))
        (:<
          (Pawn|SetControlRotation (Pawn|GetController) (Math|Rotator|MakeRotator 0.0 0.0 1.8e+02)))))))

(event EventBeginPlay
  (Utilities|FlowControl|Sequence
    (:then_0
      (CallFunction|DisablePlayer))
    (:then_1
      (Sprite|SetFlipbook (Variables|Default|GetSprite) "/Game/Assets/Flipbooks/FB_GolemBall.FB_GolemBall"))))

(event Collision|EventActorBeginOverlap
  (params (OtherActor :type Actor%20Object%20Reference)))

(event EventTick
  (params (DeltaSeconds :type Float%20%28single-precision%29))
  (bind _returnvalue (Transformation|GetActorLocation))
  ;[1 1 1] Update Camera Location
  (Transformation|SetWorldLocation (Variables|Default|GetSpringArm) (Math|Vector|MakeVector (Math|Float|SnapToGrid(Float) (.x _returnvalue) 4.0) 0.0 (Math|Float|SnapToGrid(Float) (+ (.z _returnvalue) 2e+02) 4.0)) false false)
  (CallFunction|UpdateDirection)
  (if (Variables|Default|GetIsEnabled)
    (Sprite|SetFlipbook (Variables|Default|GetSprite) "/Game/Assets/Flipbooks/FB_PlayerB_Idle.FB_PlayerB_Idle")))

(event Input|ActionEvents|InputActionJump
  (params (Key :type Key%20Structure :default "None"))
  (:Pressed
    ;[1 1 1] Movement
    (Character|Jump))
  (:Released
    (Character|StopJumping)))

(event Input|ActionEvents|InputActionSprint
  (params (Key :type Key%20Structure :default "None"))
  (bind _charactermovement (Variables|Character|GetCharacterMovement))
  ;[1 1 1] Movement
  (:Pressed
    (Variables|/Script/Engine.CharacterMovementComponent|SetMaxWalkSpeed _charactermovement (Variables|Default|GetSprintSpeed)))
  (:Released
    (Variables|/Script/Engine.CharacterMovementComponent|SetMaxWalkSpeed _charactermovement (Variables|Default|GetWalkSpeed))))

(event Input|AxisEvents|InputAxisMove
  (params (AxisValue :type Float%20%28single-precision%29))
  ;[1 1 1] Movement
  (Pawn|Input|AddMovementInput "1.000000, 0, 0" AxisValue false))

(event Input|KeyboardEvents|T
  (params (Key :type Key%20Structure :default "None"))
  (:Pressed
    (Utilities|FlowControl|FlipFlop
      (:A
        (Utilities|FlowControl|Sequence
          (:then_0
            (CallFunction|DisablePlayer))
          (:then_1
            (Sprite|SetFlipbook (Variables|Default|GetSprite) "/Game/Assets/Flipbooks/FB_GolemBall.FB_GolemBall"))))
      (:B
        (Utilities|FlowControl|Sequence
          (:then_0
            (CallFunction|EnablePlayer))
          (:then_1
            (Sprite|SetFlipbook (Variables|Default|GetSprite) "/Game/Assets/Flipbooks/FB_PlayerB_Idle.FB_PlayerB_Idle")))))))

(event Input|KeyboardEvents|C
  (params (Key :type Key%20Structure :default "None"))
  (:Pressed
    ;[1 1 1] Change Character
    (bind _returnvalue (Actor|GetActorOfClass "/Game/Blueprints/BP_PlayerA.BP_PlayerA_C"))
    (Pawn|Possess (Game|GetPlayerController 0) _returnvalue)))

(fn ConstructionScript)

(fn DisablePlayer
  (Pawn|Components|CharacterMovement|DisableMovement (Variables|Character|GetCharacterMovement))
  (Variables|Default|SetIsEnabled false))

(fn EnablePlayer
  (Pawn|Components|CharacterMovement|SetMovementMode (Variables|Character|GetCharacterMovement) "MOVE_Walking" 0)
  (Variables|Default|SetIsEnabled true))