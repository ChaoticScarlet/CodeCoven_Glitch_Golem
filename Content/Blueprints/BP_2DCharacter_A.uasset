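; Playable 2D character A, one of at least two characters the player can switch between.
; Its construction script runs the parent's, then sets its own walk speed, sprint speed and max health.
; Crouch input toggles crouching, and C makes the first player controller possess the BP_2DCharacter_B found in the level if that character's IsEnabled flag is set.
; BeginPlay only calls the parent, and Tick and overlap are disabled stubs.
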(event EventBeginPlay
  (|CallParentFunction))

(event Collision|EventActorBeginOverlap
  (params (OtherActor :type Actor%20Object%20Reference))
  (|CallParentFunction OtherActor) ; This node is disabled and will not be called.\nDrag off pins to build functionality.
)

(event EventTick
  (params (DeltaSeconds :type Float%20%28single-precision%29))
  (|CallParentFunction DeltaSeconds) ; This node is disabled and will not be called.\nDrag off pins to build functionality.
)

(event Input|ActionEvents|InputActionCrouch
  (params (Key :type Key%20Structure))
  (:Pressed
    ;[1 1 1] Movement
    (Character|Crouch))
  (:Released
    (Character|UnCrouch)))

(event Input|KeyboardEvents|C
  (params (Key :type Key%20Structure))
  (:Pressed
    ;[1 1 1] Change Character
    (bind _returnvalue (Actor|GetActorOfClass "/Game/Blueprints/BP_2DCharacter_B.BP_2DCharacter_B_C"))
    (if (Variables|/Game/Blueprints/BP_2DCharacter_B.BP_2DCharacter_B_C|GetIsEnabled _returnvalue)
      (Pawn|Possess (Game|GetPlayerController 0) _returnvalue))))

(fn ConstructionScript
  (|CallParentFunction)
  (Variables|Default|SetWalkSpeed 8e+02)
  (Variables|Default|SetSprintSpeed 2e+03)
  (Variables|Default|SetMaxHealth 1e+02))