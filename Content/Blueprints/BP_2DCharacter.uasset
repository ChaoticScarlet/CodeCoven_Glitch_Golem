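; Player character for a 2D side-scroller that moves along X with jump and sprint, takes damage and toggles a pause menu.
; Each tick it grid-snaps the spring arm to its location for a pixel-aligned camera and flips control yaw by horizontal velocity.
; BeginPlay fills health and creates the HUD; at zero health the actor destroys itself, and Destroyed asks BP_GameMode to respawn the player.
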(event Custom|UpdateDirection
  (Utilities|IsValid (Pawn|GetController)
    (:Is%20Valid
      (CallFunction|UpdateCharacterDirection))))

(event Custom|Death
  ;[1 1 1] Death
  (Actor|DestroyActor))

(event EventBeginPlay
  (CallFunction|SetHealth))

(event Collision|EventActorBeginOverlap
  (params (OtherActor :type Actor%20Object%20Reference)))

(event EventTick
  (params (DeltaSeconds :type Float%20%28single-precision%29))
  (CallFunction|UpdateCameraLocation)
  (CallFunction|UpdateDirection))

(event Game|Damage|EventAnyDamage
  (params (Damage :type Float%20%28single-precision%29) (DamageType :type Damage%20Type%20Object%20Reference) (InstigatedBy :type Controller%20Object%20Reference) (DamageCauser :type Actor%20Object%20Reference))
  ;[1 1 1] Taking Damage
  (Variables|Default|SetCurrentHealth (- (Variables|Default|GetCurrentHealth) Damage))
  (if (<= (Variables|Default|GetCurrentHealth) 0.0)
    (CallFunction|Death)))

(event EventDestroyed
  ;[1 1 1] Death
  (bind _asbp_game_mode (Utilities|Casting|CastToBP_GameMode (Game|GetGameMode)))
  (Default|RespawnPlayerA _asbp_game_mode))

(event Input|ActionEvents|InputActionJump
  (params (Key :type Key%20Structure :default "None"))
  (:Pressed
    ;[1 1 1] Movement
    (Character|Jump))
  (:Released
    (Character|StopJumping)))

(event Input|ActionEvents|InputActionSprint
  (params (Key :type Key%20Structure :default "None"))
  (bind _charactermovement (Variables|Character|GetCharacterMovement))
  (:Pressed
    ;[1 1 1] Movement
    (Variables|/Script/Engine.CharacterMovementComponent|SetMaxWalkSpeed _charactermovement (Variables|Default|GetSprintSpeed)))
  (:Released
    (Variables|/Script/Engine.CharacterMovementComponent|SetMaxWalkSpeed _charactermovement (Variables|Default|GetWalkSpeed))))

(event Input|ActionEvents|InputActionPause
  (params (Key :type Key%20Structure :default "None"))
  (:Pressed
    ;[1 1 1] Pause Menu
    (if (Variables|Default|GetIsPauseMenuOpen)
      (CallFunction|ClosePauseMenu)
      (else
        (CallFunction|OpenPauseMenu)))))

(event Input|AxisEvents|InputAxisMove
  (params (AxisValue :type Float%20%28single-precision%29))
  ;[1 1 1] Movement
  (Pawn|Input|AddMovementInput "1.000000, 0, 0" AxisValue false))

(fn ConstructionScript)

(fn SetHealth
  (Variables|Default|SetCurrentHealth (Variables|Default|GetMaxHealth))
  (bind _returnvalue (UserInterface|CreateWidget "/Game/UI/WBP_HUD.WBP_HUD_C" (Game|GetPlayerController 0)))
  (UserInterface|Viewport|AddtoViewport _returnvalue 0))

(fn UpdateCameraLocation
  (bind _returnvalue (Transformation|GetActorLocation))
  (Transformation|SetWorldLocation (Variables|Default|GetSpringArm) (Math|Vector|MakeVector (Math|Float|SnapToGrid(Float) (.x _returnvalue) 4.0) 0.0 (Math|Float|SnapToGrid(Float) (+ (.z _returnvalue) 1e+02) 4.0)) false false))

(fn OpenPauseMenu
  (bind _returnvalue (Game|GetPlayerController 0))
  (Variables|Default|SetIsPauseMenuOpen true)
  (bind _returnvalue_2 (UserInterface|CreateWidget "/Game/UI/WBP_PauseMenu.WBP_PauseMenu_C" _returnvalue))
  (bind _output_get (Variables|Default|SetPauseMenuWidget _returnvalue_2))
  (UserInterface|Viewport|AddtoViewport _output_get 0)
  (Input|SetInputModeGameandUI _returnvalue (Variables|Default|GetPauseMenuWidget) "DoNotLock" true)
  (Variables|/Script/Engine.PlayerController|SetbShowMouseCursor (Game|GetPlayerController 0) true)
  (Game|SetGamePaused true))

(fn ClosePauseMenu
  (Variables|Default|SetIsPauseMenuOpen false)
  (Widget|RemovefromParent (Variables|Default|GetPauseMenuWidget))
  (Game|SetGamePaused false)
  (Input|SetInputModeGameOnly)
  (Variables|/Script/Engine.PlayerController|SetbShowMouseCursor (Game|GetPlayerController 0) false))

(fn UpdateCharacterDirection
  (Math|Float|CompareFloat (.X (Math|Vector|BreakVector (Variables|/Script/Engine.MovementComponent|GetVelocity (Variables|Character|GetCharacterMovement)))) 0.0
    (:>
      (Pawn|SetControlRotation (Pawn|GetController) (Math|Rotator|MakeRotator 0.0 0.0 0.0)))
    (:<
      (Pawn|SetControlRotation (Pawn|GetController) (Math|Rotator|MakeRotator 0.0 0.0 1.8e+02)))))