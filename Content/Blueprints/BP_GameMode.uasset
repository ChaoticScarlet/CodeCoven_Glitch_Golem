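; Game mode that handles respawning the first 2D character and handing control to the second one, the Golem.
; Tick compares acquired Golem fires to the total; on a match it enables the placed BP_2DCharacter_B, possesses it and zeroes the total to avoid retriggering.
; RespawnPlayerA spawns a new BP_2DCharacter_A at the stored start transform and has the player controller possess it.
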(event Custom|RespawnPlayerA
  (bind _startlocation (Variables|Default|GetStartLocation))
  ;[1 1 1] Respawn
  (bind _returnvalue (Game|SpawnActorfromClass "/Game/Blueprints/BP_2DCharacter_A.BP_2DCharacter_A_C" (Math|Transform|MakeTransform (.location _startlocation) (.rotation _startlocation) (.scale _startlocation)) "Undefined" 0 0))
  (Pawn|Possess (Game|GetPlayerController 0) _returnvalue))

(event EventBeginPlay)

(event EventTick
  (params (DeltaSeconds :type Float%20%28single-precision%29))
  ;[1 1 1] Activate Golem
  (if (== (Variables|Default|GetGolemFiresAdquired) (Variables|Default|GetTotalGolemFires))
    (bind _returnvalue (Actor|GetActorOfClass "/Game/Blueprints/BP_2DCharacter_B.BP_2DCharacter_B_C"))
    (Default|EnablePlayer _returnvalue)
    (Pawn|Possess (Game|GetPlayerController 0) _returnvalue)
    (Variables|Default|SetTotalGolemFires 0)))

(fn ConstructionScript)